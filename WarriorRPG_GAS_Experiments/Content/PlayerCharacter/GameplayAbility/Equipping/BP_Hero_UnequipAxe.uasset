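; Gameplay ability that unequips the hero's axe, playing the unequip montage and ending when it finishes or is interrupted.
; It clears the equipped weapon tag, then waits for the unequip gameplay event to snap the axe to the back socket.
; It then unlinks the weapon's anim layer, removes its input mapping context and revokes the abilities it granted.
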(event `self.K2_ActivateAbility`
  (`AbilityTask_PlayMontageAndWait.CreatePlayMontageAndWaitProxy` "None" "/Game/PlayerCharacter/Montages/AM_Hero_Axe_Unequip.AM_Hero_Axe_Unequip"
    (:`then`
      (set `PawnCombatComponent.CurrentEquippedWeaponTag` (struct) (`self.GetHeroCombatComponentFromActorInfo`))
      (`AbilityTask_WaitGameplayEvent.WaitGameplayEvent` (struct :`TagName` "Player.Event.Unequip.Axe") null
        (:`EventReceived`
          (`Actor.K2_AttachToComponent` (`HeroCombatComponent.GetHeroCarriedWeaponByTag` (`self.GetHeroCombatComponentFromActorInfo`) (struct :`TagName` "Player.Weapon.Axe")) (`self.GetOwningComponentFromActorInfo`) "AxeBackSocket" "SnapToTarget" "KeepRelative" "KeepWorld" true)
          (`self.HandleUnequipWeapon` (`HeroCombatComponent.GetHeroCarriedWeaponByTag` (`self.GetHeroCombatComponentFromActorInfo`) (struct :`TagName` "Player.Weapon.Axe"))))))
    (:`OnCompleted`
      (`self.K2_EndAbility` :!label _label))
    (:`OnBlendOut`
      (goto _label))
    (:`OnInterrupted`
      (goto _label))
    (:`OnCancelled`
      (goto _label))))

(fn `HandleUnequipWeapon`
  (params (InWeaponToUnequip :type "WarriorHeroWeapon Object Reference"))
  (bind (_cachedheroweapondata_weaponanimlayertolink _cachedheroweapondata_weaponinputmappingcontext) (break `WarriorHeroWeaponData` (`self.CachedHeroWeaponData`)))
  (bind _cachedheroweapondata_weaponanimlayertolink_2 (break `WarriorHeroWeaponData` (`self.CachedHeroWeaponData`)))
  (set `self.CachedHeroWeaponData` (`WarriorHeroWeapon.HeroWeaponData` InWeaponToUnequip))
  (`|ExecutionSequence`
    (:`then_0`
      (`SkeletalMeshComponent.UnlinkAnimClassLayers` (`self.GetOwningComponentFromActorInfo`) _cachedheroweapondata_weaponanimlayertolink_2))
    (:`then_1`
      (`EnhancedInputSubsystemInterface.RemoveMappingContext` (pcsubsystem `EnhancedInputLocalPlayerSubsystem` (`self.GetHeroControllerFromActorInfo`)) _cachedheroweapondata_weaponinputmappingcontext (struct)))
    (:`then_2`
      (`WarriorAbilitySystemComponent.RemovedGrantedHeroWeaponAbilities` (`self.GetWarriorAbilitySystemComponentFromActorInfo`) (`WarriorHeroWeapon.GetGrantedAbilitySpecHandles` (`local.InWeaponToUnequip`))))))